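; BP_SnakeController is a controller that feeds player movement input to the snake pawn.
; On BeginPlay it adds the snake mapping context to the Enhanced Input subsystem.
; The Move action's Triggered event casts the controlled pawn to BP_SnakePawn and passes the X and Y values to its OnMove.
; On possession it prints a debug string naming itself and the possessed pawn.
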(event `EnhancedInput|/Game/Input/Move`
  (params (ActionValue :type "Vector2D Structure") (ElapsedSeconds :type "Float (double-precision)") (TriggeredSeconds :type "Float (double-precision)") (InputAction :type "InputAction Object Reference" :default "/Game/Input/Move.Move"))
  (:`Triggered`
    (bind _asbp_snake_pawn (cast `/Game/Blueprint/BP_SnakePawn` (`self.K2_GetPawn`)))
    (`PlayerPawnBase.OnMove` _asbp_snake_pawn ActionValue_X ActionValue_Y)))

(event `self.ReceiveBeginPlay`
  (message `EnhancedInputSubsystemInterface.AddMappingContext` (subsystem `EnhancedInputLocalPlayerSubsystem`) "/Game/Input/SnakeMappingContext.SnakeMappingContext" 0 (struct)))

(event `self.ReceivePossess`
  (params (PossessedPawn :type "Pawn Object Reference"))
  (`KismetSystemLibrary.PrintString` (`KismetStringLibrary.Concat_StrStr` (`KismetSystemLibrary.GetDisplayName` self) (`self.PrintString`) (`KismetSystemLibrary.GetDisplayName` PossessedPawn)) true true (struct :`G` 0.66 :`B` 1.0 :`A` 1.0) 100.0))

(fn `UserConstructionScript`)