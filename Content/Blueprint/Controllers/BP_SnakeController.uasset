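; Player controller for a snake game that routes Enhanced Input movement to the snake pawn and handles death and restart.
; On possession it caches the pawn, adds the snake mapping context and prints a debug message.
; Game state delegates drive the rest: death stops pawn tick and shows the cursor.
; Restart hides the cursor, teleports the pawn to player start, zeroes the controller's actor rotation and resumes tick.
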(event `EnhancedInput|/Game/Input/Move`
  (params (ActionValue :type "Vector2D Structure") (ElapsedSeconds :type "Float (double-precision)") (TriggeredSeconds :type "Float (double-precision)") (InputAction :type "InputAction Object Reference" :default "/Game/Input/Move.Move"))
  ; Movement code
  (:`Triggered`
    (bind _asbp_snake_pawn (cast `/Game/Blueprint/Pawns/BP_SnakePawn` (`self.K2_GetPawn`)))
    (`PlayerPawnBase.OnMove` _asbp_snake_pawn ActionValue_X ActionValue_Y)))

(event `self.ReceivePossess`
  (params (PossessedPawn :type "Pawn Object Reference"))
  ; Add Mapping Context with debugs
  (bind _asplayer_pawn_base (cast `PlayerPawnBase` PossessedPawn))
  (set `self.Possessed Pawn` _asplayer_pawn_base)
  (message `EnhancedInputSubsystemInterface.AddMappingContext` (subsystem `EnhancedInputLocalPlayerSubsystem`) "/Game/Input/SnakeMappingContext.SnakeMappingContext" 0 (struct))
  (`KismetSystemLibrary.PrintString` (`KismetStringLibrary.Concat_StrStr` (`KismetSystemLibrary.GetDisplayName` self) (`self.PrintString`) (`KismetSystemLibrary.GetDisplayName` PossessedPawn)) true true (struct :`G` 0.66 :`B` 1.0 :`A` 1.0) 100.0))

(event `self.ReceiveBeginPlay`
  ; Event Listeners
  (bind _assnake_game_state (cast `SnakeGameState` (`GameplayStatics.GetGameState`)))
  (bind _returnvalue (`SnakeGameState.GetDelegateData` _assnake_game_state))
  (add `DelegateData.OnPlayerDied` _returnvalue (delegate `OnPlayerDied_Event`))
  (add `DelegateData.OnGameRestarted` _returnvalue (delegate `OnGameRestarted_Event`)))

(event `OnPlayerDied_Event`
  ; Event Listeners
  (`self.SetActorTickEnabled` (`self.Possessed Pawn`) false)
  (set `self.bShowMouseCursor` true))

(event `OnGameRestarted_Event`
  (bind _possessed_pawn (`self.Possessed Pawn`))
  ; Event Listeners
  (set `self.bShowMouseCursor` false)
  (`self.K2_SetActorLocation` _possessed_pawn (`self.K2_GetActorLocation` (`GameModeBase.K2_FindPlayerStart` (`GameplayStatics.GetGameMode`) self "")) false true)
  (`self.K2_SetActorRotation` (struct) true)
  (`self.SetActorTickEnabled` _possessed_pawn true))

(fn `UserConstructionScript`)